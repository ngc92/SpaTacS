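; Player pawn that adds the single-ship HUD on BeginPlay and draws 3D position markers for the ship selected in PlayerPawnController.
; Each tick with a valid selection, it places markers at the controller's target position and the ship's desired propulsion destination; without one, it hides the target marker.
; Marker bases, plus one under the ship, are projected onto a horizontal reference plane offset from the pawn's height.
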(event `self.ReceiveBeginPlay`
  (bind _returnvalue (`|CreateWidget` "/Game/SingleShipHUD.SingleShipHUD_C"))
  (`UserWidget.AddToViewport` _returnvalue 0)
  (bind _asplayer_pawn_controller (cast `PlayerPawnController` (`self.GetController`)))
  (set `self.PlayerPawnController` _asplayer_pawn_controller))

(event `self.ReceiveTick`
  (params (DeltaSeconds :type "Float (single-precision)"))
  (bind _targetmarker (`self.TargetMarker`))
  (bind _selectedship (`PlayerPawnController.SelectedShip` (`self.PlayerPawnController`)))
  (`/Engine/EditorBlueprintResources/StandardMacros.IsValid` _selectedship
    (:`Is Valid`
      (`SceneComponent.SetVisibility` _targetmarker true true)
      (`self.Set 3D Marker` (`PlayerPawnController.GetTargetPosition` (`self.PlayerPawnController`)) (`self.TargetMarkerVisual`) (`self.TargetMarkerBase`))
      (`self.Set Ship Base Marker` (`self.K2_GetActorLocation` _selectedship))
      (`self.Set 3D Marker` (`PropulsionControlComponent.DesiredPosition` (`StarShip.Propulsion` _selectedship)) (`self.ShipDestinationMarker`) (`self.ShipDestinationMarkerBase`)))
    (:`Is Not Valid`
      (`SceneComponent.SetVisibility` _targetmarker false true))))

(fn `Project To View Plane`
  (params (`World Location` :type "Vector Structure"))
  (returns (`View Plane Location` :type "Vector Structure"))
  (return (`KismetMathLibrary.MakeVector` (.x `World Location`) (.y `World Location`) (+ (.z (`self.K2_GetActorLocation`)) (`PlayerPawnController.ReferencePlaneZ` (`self.PlayerPawnController`))))))

(fn `Set 3D Marker`
  (params (TargetLocation :type "Vector Structure") (Marker :type "SceneComponent Object Reference") (Base :type "SceneComponent Object Reference"))
  (`SceneComponent.K2_SetWorldLocation` Marker TargetLocation false true)
  (`SceneComponent.K2_SetWorldLocation` Base (`self.Project To View Plane` TargetLocation) false true))

(fn `Set Ship Base Marker`
  (params (TargetLocation :type "Vector Structure"))
  (`SceneComponent.K2_SetWorldLocation` (`self.ShipMarkerBase`) (`self.Project To View Plane` TargetLocation) false true))

(fn `UserConstructionScript`)